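; Game mode for Voloble that runs a sequence of streamed levels in which the player controls a roller and collects blobs.
; The base map passes in levels, spawns and an idle camera, then a hold, check, transition loop streams each level, spawns the roller and shows the HUD.
; Reaching a goal despawns the roller, unloads the level and re-enters the loop, which returns to the main menu after the last level.
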(event `InitialiseGame`
  (params (Levels :type "Map of Integer to Name") (LevelSpawns :type "Map of Integer to Transform Structure") (IdleCam :type "CameraActor Object Reference"))
  ;[1 1 1] Initialise the game. Obtain level data from base map, save and then begin iterating through levels.
  (`KismetSystemLibrary.PrintString` "Initialised Game")
  (bind _output_get (set `self.Levels` Levels))
  (bind _output_get_2 (set `self.LevelTotal` (`BlueprintMapLibrary.Map_Length` _output_get)))
  (`KismetSystemLibrary.PrintString` "Levels Loaded")
  (`KismetSystemLibrary.PrintString` (`KismetStringLibrary.Conv_IntToString` _output_get_2))
  (set `self.IdleCamera` IdleCam)
  (`KismetSystemLibrary.PrintString` "Got idle cam")
  (set `self.LevelSpawns` LevelSpawns)
  (`KismetSystemLibrary.PrintString` "Loaded level spawn data")
  (`self.LevelHoldEvent`))

(event `LevelTransitionEvent`
  (`GameplayStatics.LoadStreamLevel` (`BlueprintMapLibrary.Map_Find` (`self.Levels`) (`self.CurrentLevel`)) true)
  (bind _returnvalue (`|CreateWidget` "/Game/UI/In-GameAnimations/LevelIntro.LevelIntro_C"))
  (`UserWidget.AddToViewport` _returnvalue 0)
  (`KismetSystemLibrary.Delay` 1.8)
  (bind _asgm_voloble_pc (cast `/Game/Game/Voloble/Gamemode/GM_Voloble_PC` (`GameplayStatics.GetPlayerController` 0)))
  (`/Game/Game/Voloble/Gamemode/GM_Voloble_PC.SpawnRoller` _asgm_voloble_pc (`BlueprintMapLibrary.Map_Find` (`self.LevelSpawns`) (`self.CurrentLevel`)))
  (`self.ShowHUD`))

(event `CheckNextLevelEvent`
  (if (>= (`self.CurrentLevel`) (`self.LevelTotal`))
    (bind _asvoloble (cast `/Game/Game/Voloble/Voloble` (`GameplayStatics.GetGameInstance`)))
    (`/Game/Game/Voloble/Voloble.MainMenu` _asvoloble)
    (else
      (set `self.CurrentLevel` (+ (`self.CurrentLevel`) 1))
      (`self.LevelTransitionEvent`))))

(event `LevelHoldEvent`
  (`PlayerController.SetViewTargetWithBlend` (`GameplayStatics.GetPlayerController` 0) (`self.IdleCamera`) 0.0 "VTBlend_Linear" 0.0 false)
  (`KismetSystemLibrary.Delay` 1.0)
  (`self.CheckNextLevelEvent`))

(event `LevelGoalEvent`
  (`self.HideHUD`)
  (bind _returnvalue (`|CreateWidget` "/Game/UI/In-GameAnimations/Goal.Goal_C"))
  (`UserWidget.AddToViewport` _returnvalue 0)
  (`KismetSystemLibrary.Delay` 0.5)
  (bind _asgm_voloble_pc (cast `/Game/Game/Voloble/Gamemode/GM_Voloble_PC` (`GameplayStatics.GetPlayerController` 0)))
  (`/Game/Game/Voloble/Gamemode/GM_Voloble_PC.DespawnRoller` _asgm_voloble_pc)
  (`GameplayStatics.UnloadStreamLevel` (`BlueprintMapLibrary.Map_Find` (`self.Levels`) (`self.CurrentLevel`)))
  (`KismetSystemLibrary.Delay` 1.5)
  (`self.LevelHoldEvent`))

(event `AddBlobsEvent`
  (bind _huddata (`self.HUDdata`))
  (set `self.Blobs` (+ (`self.Blobs`) 1))
  (`GameplayStatics.PlaySound2D` "/Game/Sound/SFX/ding_Cue.ding_Cue" 1.0 1.0 0.0 null null)
  (`UserWidget.PlayAnimation` _huddata (`/Game/UI/HUD.BlobGot` _huddata) 0.0 1 "Forward" 1.0 false))

(event `ShowHUD`
  (bind _returnvalue (`|CreateWidget` "/Game/UI/HUD.HUD_C"))
  (`UserWidget.AddToViewport` _returnvalue 0)
  (`KismetSystemLibrary.PrintString` "HUD Displayed" true true (struct :`R` 1.0 :`G` 0.030354 :`B` 0.070155 :`A` 1.0))
  (set `self.HUDdata` _returnvalue))

(event `HideHUD`
  (`/Game/UI/HUD.RemoveHUD` (stale `ShowHUD` _returnvalue))
  (`KismetSystemLibrary.PrintString` "HUD Removed" true true (struct :`R` 1.0 :`G` 0.030354 :`B` 0.070155 :`A` 1.0)))

(fn `UserConstructionScript`)